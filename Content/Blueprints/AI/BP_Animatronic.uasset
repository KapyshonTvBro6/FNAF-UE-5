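; Animatronic enemy that patrols between BP_Local rooms and kills the player on contact.
; Patrol moves to a random different room, repeating whether the move succeeds or fails.
; The See volume triggers a one-shot move toward the player's position on entering and leaving; the Dead volume shows game over, then quits.
; Line-of-sight, chase state and aggression logic is inactive: its events are empty stubs and the code is disconnected.
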(event `self.ReceiveBeginPlay`
  ; Инициализация
  (set `self.PlayerRef` (`GameplayStatics.GetPlayerCharacter` 0))
  (set `CharacterMovementComponent.MaxWalkSpeed` (`self.ChaseSpeed`) (`self.CharacterMovement`))
  (bind _outactors (`GameplayStatics.GetAllActorsOfClass` "/Game/Blueprints/AI/BP_Local.BP_Local_C"))
  (for _array_element _outactors
    (`KismetArrayLibrary.Array_Set` (`self.Rooms`) (`/Game/Blueprints/AI/BP_Local.ID_Room` _array_element) _array_element true))
  (`self.StartPatrol`))

(event `KillPlayer`
  ; СИСТЕМА УБИЙСТВА ИГРОКА
  (if (`KismetSystemLibrary.IsValid` (`self.PlayerRef`))
    (if (`self.Near`)
      (cast `/Game/FirstPerson/Blueprints/BP_FirstPersonGameMode` (`GameplayStatics.GetGameMode`))
      (if (`self.IsFinalChaseActive`)
        (`KismetSystemLibrary.PrintString` "💀 ВЫ НЕ СМОГЛИ УБЕЖАТЬ..." true true (struct :`R` 1.0 :`A` 1.0) 5.0)
        (else
          (`KismetSystemLibrary.PrintString` "💀 GAME OVER" true true (struct :`R` 1.0 :`A` 1.0))))
      (`KismetSystemLibrary.Delay` 2.0)
      (`KismetSystemLibrary.QuitGame` (`GameplayStatics.GetPlayerController` 0) "Quit"))))

(event `self.Dead.OnComponentBeginOverlap`
  (params (OverlappedComponent :type "PrimitiveComponent Object Reference") (OtherActor :type "Actor Object Reference") (OtherComp :type "PrimitiveComponent Object Reference") (OtherBodyIndex :type Integer) (bFromSweep :type Boolean) (SweepResult :type "HitResult Structure (by ref)"))
  ; СИСТЕМА УБИЙСТВА ИГРОКА
  (cast `/Game/FirstPerson/Blueprints/BP_FirstPersonCharacter` OtherActor)
  (set `self.Near` true)
  (`self.KillPlayer`))

(event `self.Dead.OnComponentEndOverlap`
  (params (OverlappedComponent :type "PrimitiveComponent Object Reference") (OtherActor :type "Actor Object Reference") (OtherComp :type "PrimitiveComponent Object Reference") (OtherBodyIndex :type Integer))
  ; СИСТЕМА УБИЙСТВА ИГРОКА
  (cast `/Game/FirstPerson/Blueprints/BP_FirstPersonCharacter` OtherActor)
  (set `self.Near` false)
  (`self.KillPlayer`))

(event `StartPatrol`
  ; StartPatrol
  (bind _returnvalue (`KismetMathLibrary.RandomIntegerInRange` 0 (`KismetArrayLibrary.Array_LastIndex` (`self.Rooms`)) :!label _label))
  (if (== _returnvalue (`self.IDRoom`))
    (`KismetSystemLibrary.Delay` 0.2)
    (goto _label)
    (else
      (set `self.IDRoom` _returnvalue)
      (bind _output_get (set `self.CurrentTargetLocation` (`self.K2_GetActorLocation` (`|GetArrayItem` (`self.Rooms`) (`self.IDRoom`)))))
      (`|AIMoveTo` self _output_get null 100.0
        (:`OnSuccess`
          _)
        (:`OnFail`
          _))
      (`self.StartPatrol`))))

(event `ChaseUpdateTimer`
  (bind (_currenttargetlocation_x _currenttargetlocation_y) (`KismetMathLibrary.BreakVector` (`self.CurrentTargetLocation`)))
  (set `self.CurrentTargetLocation` (`self.K2_GetActorLocation` (`GameplayStatics.GetPlayerPawn` 0)))
  (`|AIMoveTo` self (`KismetMathLibrary.MakeVector` _currenttargetlocation_x _currenttargetlocation_y) null 100.0 true))

(event `self.ReceiveTick`
  (params (DeltaSeconds :type "Float (single-precision)"))
  ; Проверка достижения точки
)

(event `StartChase`
  ; СИСТЕМА ПРЕСЛЕДОВАНИЯ
)

(event `StopChase`
  ; СИСТЕМА ПРЕСЛЕДОВАНИЯ
)

(event `OnPlayerSpotted`
  ; СИСТЕМА АГРЕССИИ
)

(event `OnPlayerLost`
  ; СИСТЕМА АГРЕССИИ
)

(event `CheckPlayerVisibility`
  ; СИСТЕМА ОБНАРУЖЕНИЯ ИГРОКА
)

(event `self.See.OnComponentBeginOverlap`
  (params (OverlappedComponent :type "PrimitiveComponent Object Reference") (OtherActor :type "Actor Object Reference") (OtherComp :type "PrimitiveComponent Object Reference") (OtherBodyIndex :type Integer) (bFromSweep :type Boolean) (SweepResult :type "HitResult Structure (by ref)"))
  ; СИСТЕМА ОБНАРУЖЕНИЯ ИГРОКА
  (cast `/Game/FirstPerson/Blueprints/BP_FirstPersonCharacter` OtherActor)
  (set `self.CanSeePlayer` true)
  (`self.ChaseUpdateTimer`))

(event `self.See.OnComponentEndOverlap`
  (params (OverlappedComponent :type "PrimitiveComponent Object Reference") (OtherActor :type "Actor Object Reference") (OtherComp :type "PrimitiveComponent Object Reference") (OtherBodyIndex :type Integer))
  ; СИСТЕМА ОБНАРУЖЕНИЯ ИГРОКА
  (cast `/Game/FirstPerson/Blueprints/BP_FirstPersonCharacter` OtherActor)
  (set `self.CanSeePlayer` false)
  (`self.ChaseUpdateTimer`))

(fn `DecreaseAggression`
  (if (not (`self.CanSeePlayer`))
    (bind _output_get (set `self.AggressionLevel` (- (* (`self.AggressionIncreaseRate`) 0.1) (`self.AggressionLevel`))))
    (`KismetMathLibrary.Clamp` (`KismetMathLibrary.FTrunc` _output_get) 0 100)
    (if (and (<= (`self.AggressionLevel`) 0.0) (`self.IsChasing`))
      _)))

(fn `IncreaseAggression`
  (if (`self.CanSeePlayer`)
    (bind _output_get (set `self.AggressionLevel` (+ (* (`self.AggressionIncreaseRate`) 0.1) (`self.AggressionLevel`))))
    (`KismetMathLibrary.Clamp` (`KismetMathLibrary.FTrunc` _output_get) 0 100)
    (if (and (>= (`self.AggressionLevel`) (`self.AggressionThreshold`)) (`self.IsChasing`))
      (`self.StartChase`))))

(fn `UserConstructionScript`)