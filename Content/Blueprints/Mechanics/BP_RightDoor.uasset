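; BP_RightDoor is a door that toggles open and closed, tied to the level's power system.
; ToggleDoor flips the closed state while power remains, setting a target height and playing a 2D sound.
; Tick interpolates the door mesh's Z toward that target with FInterpTo.
; When BP_PowerSystem, found on BeginPlay, runs out, Tick forces the target open and plays the sound once via a latch flag, leaving IsClosed unchanged.
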(event `self.ReceiveBeginPlay`
  (bind _returnvalue (`GameplayStatics.GetActorOfClass` "/Game/Blueprints/Mechanics/BP_PowerSystem.BP_PowerSystem_C"))
  (set `self.PowerSystemRef` _returnvalue))

(event `ToggleDoor`
  (if (not (`/Game/Blueprints/Mechanics/BP_PowerSystem.IsOutOfPower` (`self.PowerSystemRef`)))
    (bind _output_get (set `self.IsClosed` (not (`self.IsClosed`))))
    (if _output_get
      (set `self.TargetZ` (`self.ClosedZ`))
      (else
        (set `self.TargetZ` (`self.OpenZ`))))
    (`GameplayStatics.PlaySound2D` "/Game/AUDIO/sfxbible-12478.sfxbible-12478" 1.0 1.0 0.0 null null :!label _label)))

(event `self.ReceiveTick`
  (params (DeltaSeconds :type "Float (single-precision)"))
  (bind _returnvalue (`SceneComponent.GetRelativeTransform` (`self.Door Mesh`)))
  (`SceneComponent.K2_SetRelativeLocation` (`self.Door Mesh`) (`KismetMathLibrary.MakeVector` (.x (.location _returnvalue)) (.y (.location _returnvalue)) (`KismetMathLibrary.FInterpTo` (.z (.location _returnvalue)) (`self.TargetZ`) DeltaSeconds (`self.InterpSpeed`))) false false)
  (if (`/Game/Blueprints/Mechanics/BP_PowerSystem.IsOutOfPower` (`self.PowerSystemRef`))
    (set `self.TargetZ` (`self.OpenZ`))
    (if (not (`self.NewVar`))
      (set `self.NewVar` true)
      (goto _label))
    (else
      (set `self.NewVar` false))))

(fn `UserConstructionScript`)