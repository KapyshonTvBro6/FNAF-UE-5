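; Right-side light actor that switches a spotlight on and off, gated by the game's power system.
; On BeginPlay it finds and caches the BP_PowerSystem actor in the level.
; ToggleLight flips IsOn and sets the SpotLight's visibility to match, doing nothing while the power system is out of power.
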(event `self.ReceiveBeginPlay`
  (bind _returnvalue (`GameplayStatics.GetActorOfClass` "/Game/Blueprints/Mechanics/BP_PowerSystem.BP_PowerSystem_C"))
  (set `self.PowerSystemRef` _returnvalue))

(event `ToggleLight`
  (if (not (`/Game/Blueprints/Mechanics/BP_PowerSystem.IsOutOfPower` (`self.PowerSystemRef`)))
    (bind _output_get (set `self.IsOn` (not (`self.IsOn`))))
    (if _output_get
      (`SceneComponent.SetVisibility` (`self.SpotLight`) true false)
      (else
        (`SceneComponent.SetVisibility` (`self.SpotLight`) false false)))))

(fn `UserConstructionScript`)