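; Power system actor that manages an energy reserve drained by closed doors and active lights on the left and right.
; BeginPlay finds the door and light actors; Tick sums their drain rates and subtracts from PowerLevel only while CAM08LightOn is true.
; Remaining energy prints as debug text.
; PowerOutage opens doors and switches off lights, but its zero check sits inside a greater-than-zero branch, so Tick never reaches it.
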(event `self.ReceiveBeginPlay`
  (bind _returnvalue (`GameplayStatics.GetActorOfClass` "/Game/Blueprints/Mechanics/BP_RightDoor.BP_RightDoor_C"))
  (set `self.RigthDoor` _returnvalue)
  (bind _returnvalue_2 (`GameplayStatics.GetActorOfClass` "/Game/Blueprints/Mechanics/BP_LeftDoor.BP_LeftDoor_C"))
  (set `self.LeftDoor` _returnvalue_2)
  (bind _returnvalue_3 (`GameplayStatics.GetActorOfClass` "/Game/Blueprints/Mechanics/BP_RightLight.BP_RightLight_C"))
  (set `self.RightLight` _returnvalue_3)
  (bind _returnvalue_4 (`GameplayStatics.GetActorOfClass` "/Game/Blueprints/Mechanics/BP_LeftLight.BP_LeftLight_C"))
  (set `self.LeftLight` _returnvalue_4))

(event `self.ReceiveTick`
  (params (DeltaSeconds :type "Float (single-precision)"))
  (bind _powerlevel (`self.PowerLevel`))
  (set `self.CurrentDrain` 0.0)
  ; LeftDoor
  (if (`/Game/Blueprints/Mechanics/BP_LeftDoor.IsClosed` (`self.LeftDoor`))
    (set `self.CurrentDrain` (+ (`self.CurrentDrain`) 0.2)))
  ; RightDoor
  (if (`/Game/Blueprints/Mechanics/BP_RightDoor.IsClosed` (`self.RigthDoor`))
    (set `self.CurrentDrain` (+ (`self.CurrentDrain`) 0.2)))
  ; LeftLight
  (if (`/Game/Blueprints/Mechanics/BP_LeftLight.IsOn` (`self.LeftLight`))
    (set `self.CurrentDrain` (+ (`self.CurrentDrain`) 0.02)))
  ; RightLight
  (if (`/Game/Blueprints/Mechanics/BP_RightLight.IsOn` (`self.RightLight`))
    (set `self.CurrentDrain` (+ (`self.CurrentDrain`) 0.02)))
  ; GlobalLight
  (if (`self.CAM08_LightOn`)
    (set `self.PowerLevel` (- _powerlevel (* (`self.CurrentDrain`) DeltaSeconds))))
  (if (not (not (> _powerlevel 0.0)))
    (`KismetSystemLibrary.PrintString` (`KismetTextLibrary.Conv_TextToString` (`|FormatText` "Energy {Ener}" (`self.PowerLevel`))) true true (struct :`R` 1.0 :`A` 1.0) 0.01)
    (if (== (`self.PowerLevel`) 0.0)
      (`self.PowerOutage`))))

(fn `PowerOutage`
  (set `self.IsOutOfPower` true)
  (set `/Game/Blueprints/Mechanics/BP_LeftDoor.IsClosed` false (`self.LeftDoor`))
  (set `/Game/Blueprints/Mechanics/BP_RightDoor.IsClosed` false (`self.RigthDoor`))
  (set `/Game/Blueprints/Mechanics/BP_LeftLight.IsOn` false (`self.LeftLight`))
  (set `/Game/Blueprints/Mechanics/BP_RightLight.IsOn` false (`self.RightLight`)))

(fn `UserConstructionScript`)