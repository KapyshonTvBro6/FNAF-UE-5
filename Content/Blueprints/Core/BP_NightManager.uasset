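; Night manager actor that runs the in-game clock for an animatronic survival night ending at 6 AM.
; A looping one-second timer calls UpdateClock, which advances the hour, prints it and raises animatronic AggressionLevel each hour.
; The Animatronics array holds only the single BP_Animatronic found at BeginPlay.
; At hour six, NightComplete clears its CheckMovement timer, prints the survival message and quits the game.
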(event `self.ReceiveBeginPlay`
  (bind _returnvalue (`GameplayStatics.GetActorOfClass` "/Game/Blueprints/AI/BP_Animatronic.BP_Animatronic_C"))
  (set `self.Animatronics` (`|MakeArray` _returnvalue))
  (`KismetSystemLibrary.K2_SetTimer` null "UpdateClock" 1.0 true))

(fn `NightComplete`
  (for _array_element (`self.Animatronics`)
    (`KismetSystemLibrary.K2_ClearTimer` _array_element "CheckMovement")
    (`KismetSystemLibrary.PrintString` "6 AM - You Survived!" true true (struct :`G` 1.0 :`A` 1.0) 5.0)
    (`SubmixEffectDelayStatics.SetDelayLength` (make `SubmixEffectDelaySettings` 2000.0) 3.0)
    (`KismetSystemLibrary.QuitGame` null "Quit")))

(fn `UpdateClock`
  (bind _result (`/Engine/EditorBlueprintResources/StandardMacros.IncrementFloat` (`self.TimeElapsed`))
    (:`  `
      (set `self.TimeElapsed` _result)
      (if (>= (`self.TimeElapsed`) (`self.HourDuration`))
        (bind _result_2 (`/Engine/EditorBlueprintResources/StandardMacros.IncrementInt` (`self.CurrentHour`))
          (:`  `
            (bind _output_get (set `self.CurrentHour` _result_2))
            (set `self.TimeElapsed` 0.0)
            (`KismetSystemLibrary.PrintString` (`KismetTextLibrary.Conv_TextToString` (`|FormatText` "{0} AM" _output_get)) true true (struct :`B` 1.0 :`A` 1.0) 90.0)
            (for _array_element (`self.Animatronics`)
              (set `/Game/Blueprints/AI/BP_Animatronic.AggressionLevel` (+ (`/Game/Blueprints/AI/BP_Animatronic.AggressionLevel` _array_element) 10.0) _array_element))
            (if (>= (`self.CurrentHour`) 6)
              (`self.NightComplete`))))))))

(fn `UserConstructionScript`)